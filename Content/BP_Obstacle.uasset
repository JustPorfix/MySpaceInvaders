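; BP_Obstacle is a destructible obstacle that blocks enemy projectiles and shows its remaining health by color.
; HitByProjectile decrements Health, destroys the actor once it drops below zero, and otherwise logs a message and tints the Cube.
; The tint lerps a HealthColor parameter by normalized health on a dynamic material instance created on each hit.
; Box overlap destroys incoming BP_EnemyProjectile1 actors without itself changing Health.
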(event `HitByProjectile`
  (bind _cube (`self.Cube`))
  (bind _output_get (set `self.Health` (- (`self.Health`) 1)))
  (if (< _output_get 0)
    (`self.K2_DestroyActor`)
    (else
      (`KismetSystemLibrary.LogString` "hai ancora vita fra")
      (bind _returnvalue (`PrimitiveComponent.CreateDynamicMaterialInstance` _cube 0 (`PrimitiveComponent.GetMaterial` _cube 0) "None"))
      (`MaterialInstanceDynamic.SetVectorParameterValue` _returnvalue "HealthColor" (`KismetMathLibrary.LinearColorLerp` (struct :`R` 1.0 :`B` 0.009181 :`A` 1.0) (struct :`R` 1.0 :`G` 0.13749 :`B` 0.671479 :`A` 1.0) (`KismetMathLibrary.NormalizeToRange` (`KismetMathLibrary.Conv_IntToDouble` (`self.Health`)) 0.0 5.0))))))

(event `self.Box.OnComponentBeginOverlap`
  (params (OverlappedComponent :type "PrimitiveComponent Object Reference") (OtherActor :type "Actor Object Reference") (OtherComp :type "PrimitiveComponent Object Reference") (OtherBodyIndex :type Integer) (bFromSweep :type Boolean) (SweepResult :type "HitResult Structure (by ref)"))
  (bind _asbp_enemy_projectile_1 (cast `/Game/GameFramework/Proiettili/BP_EnemyProjectile1` OtherActor))
  (`self.K2_DestroyActor` _asbp_enemy_projectile_1))

(fn `UserConstructionScript`)