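; Enemy actor that slides at a set physics velocity and periodically fires, in a style resembling Space Invaders.
; At BeginPlay it binds to every Collision actor's direction-change dispatcher, which shifts the mesh vertically by GetDown and reverses its velocity.
; A looping timer, with a cooldown randomized once at start, spawns BP_EnemyProjectile1 at the mesh.
; Moving_Down, Moving_L and Moving_R offer fixed-step root moves but are not called in these graphs.
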(event `self.ReceiveBeginPlay`
  (`|ExecutionSequence`
    (:`then_0`
      (`PrimitiveComponent.SetPhysicsLinearVelocity` (`self.Enemymesh`) (`self.Velocity`) false "None"))
    (:`then_1`
      (bind _outactors (`GameplayStatics.GetAllActorsOfClass` "/Game/GameFramework/Collider/Collision.Collision_C"))
      (for _array_element _outactors
        (add `/Game/GameFramework/Collider/Collision.OnChangeDirectioon` _array_element (delegate `OnChangeDirectioon_Event`))))
    (:`then_2`
      (`KismetSystemLibrary.K2_SetTimerDelegate` (delegate `EnemyProjectile`) (`KismetMathLibrary.RandomFloatInRange` (`self.MinCooldown`) (`self.MaxCooldown`)) true))))

(event `OnChangeDirectioon_Event`
  (bind _enemymesh (`self.Enemymesh`))
  (`SceneComponent.K2_SetWorldLocation` _enemymesh (- (`SceneComponent.K2_GetComponentLocation` _enemymesh) (* (`KismetMathLibrary.Vector_Down`) (`self.GetDown`))) false false)
  (bind _output_get (set `self.Velocity` (* (`self.Velocity`) -1.0)))
  (`PrimitiveComponent.SetPhysicsLinearVelocity` (`self.Enemymesh`) _output_get false "None"))

(event `EnemyProjectile`
  (bind _returnvalue_location (`KismetMathLibrary.BreakTransform` (`SceneComponent.K2_GetComponentToWorld` (`self.Enemymesh`))))
  (bind _returnvalue (`|SpawnActorFromClass` "/Game/GameFramework/Proiettili/BP_EnemyProjectile1.BP_EnemyProjectile1_C" (`KismetMathLibrary.MakeTransform` _returnvalue_location) "Undefined" "MultiplyWithRoot" null null)))

(fn `UserConstructionScript`)