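; BP_MyProjectile is a Space Invaders projectile that damages obstacles and kills enemies on contact.
; When its sphere begins an overlap, a sequence notifies a hit BP_Obstacle, or destroys a BP_Enemy, spawns an explosion and reports the death to BP_SpaceInvadersGameMode.
; The projectile then destroys itself, whatever it overlapped.
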(event `self.Sphere1.OnComponentBeginOverlap`
  (params (OverlappedComponent :type "PrimitiveComponent Object Reference") (OtherActor :type "Actor Object Reference") (OtherComp :type "PrimitiveComponent Object Reference") (OtherBodyIndex :type Integer) (bFromSweep :type Boolean) (SweepResult :type "HitResult Structure (by ref)"))
  (`|ExecutionSequence`
    (:`then_0`
      ;[1 1 1] - First, check if what we overlapped is an obstacle -If so, Call the function, DestroyActor
      (bind _asbp_obstacle (cast `/Game/BP_Obstacle` OtherActor))
      (`/Game/BP_Obstacle.HitByProjectile` _asbp_obstacle))
    (:`then_1`
      ;[1 1 1] - Then we check if we are overlapping an enemy
      (bind _asbp_enemy (cast `/Game/GameFramework/BP_Enemy` OtherActor))
      (`self.K2_DestroyActor` _asbp_enemy)
      (`GameplayStatics.SpawnEmitterAtLocation` "/Game/StarterContent/Particles/P_Explosion.P_Explosion" (`self.K2_GetActorLocation`) (struct) (0.5 0.5 0.5))
      (bind _asbp_space_invaders_game_mode (cast `/Game/GameFramework/BP_SpaceInvadersGameMode` (`GameplayStatics.GetGameMode`)))
      (`/Game/GameFramework/BP_SpaceInvadersGameMode.OnEnemyDeath` _asbp_space_invaders_game_mode))
    (:`then_2`
      ;[1 1 1] Destroy ourself (Projectile)
      (`self.K2_DestroyActor`))))

(fn `UserConstructionScript`)