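; BP_PlayerPawn is the player pawn, which moves along one axis, fires projectiles and triggers game over on death.
; The Move axis shifts the collision root along world Y with sweep, scaled by speed and delta time.
; Shoot spawns a projectile at a spawn point, rate-limited by a DoOnce that resets after a delay.
; Death runs once, spawning an explosion, destroying the pawn, pausing, and showing the GameOver widget and cursor.
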(event `InputAction|Shoot`
  (params (Key :type "Key Structure"))
  ;[1 1 1] Shooting system
  (:`Pressed`
    (`/Engine/EditorBlueprintResources/StandardMacros.DoOnce` false :!label _label
      (:`Completed`
        (`|SpawnActorFromClass` "/Game/GameFramework/Proiettili/BP_MyProjectile.BP_MyProjectile_C" (`KismetMathLibrary.MakeTransform` (`SceneComponent.K2_GetComponentLocation` (`self.SpawnLocationProjectile`))) "Undefined" "MultiplyWithRoot" null null)
        (`KismetSystemLibrary.Delay` 0.5)
        (goto _label :!via `Reset`)))))

(event `InputAxis|Move`
  (params (AxisValue :type "Float (single-precision)"))
  ;[1 1 1] Moovement
  (`SceneComponent.K2_SetWorldLocation` (`self.PlayerCollisionRoot`) (`KismetMathLibrary.MakeVector` (.x (`SceneComponent.K2_GetComponentLocation` (`self.PlayerCollisionRoot`))) (+ (* AxisValue (`GameplayStatics.GetWorldDeltaSeconds`) (`self.Speed`)) (.y (`SceneComponent.K2_GetComponentLocation` (`self.PlayerCollisionRoot`)))) (.z (`SceneComponent.K2_GetComponentLocation` (`self.PlayerCollisionRoot`)))) true false))

(event `self.ReceiveBeginPlay`)

(fn `Death`
  (bind _returnvalue (`GameplayStatics.GetPlayerController` 0))
  (`/Engine/EditorBlueprintResources/StandardMacros.DoOnce` false
    (:`Completed`
      (`GameplayStatics.SpawnEmitterAtLocation` "/Game/StarterContent/Particles/P_Explosion.P_Explosion" (`SceneComponent.K2_GetComponentLocation` (`self.StaticMesh`)))
      (`self.K2_DestroyActor`)
      (`GameplayStatics.SetGamePaused` true)
      (bind _returnvalue_2 (`|CreateWidget` "/Game/UI/GameOver.GameOver_C" _returnvalue))
      (bind _output_get (set `self.NewVar` _returnvalue_2))
      (`UserWidget.AddToViewport` _output_get 0)
      (set `PlayerController.bShowMouseCursor` true _returnvalue))))

(fn `UserConstructionScript`)